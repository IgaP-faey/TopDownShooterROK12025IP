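; BP_AlienSpider is an alien spider enemy that hunts and attacks the player's soldier.
; BeginPlay starts an AIMoveTo loop toward the player that retries after a short delay on success or failure.
; Tick checks soldier distance and, when close, pauses movement for an attack montage, which applies no damage here.
; Incoming damage lowers and prints health; at zero or below, it flags death, increments BP_Soldier's KillCount and stops movement.
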(event EventBeginPlay
  ;[1 0 0.9147] movement
  (if (not (Variables|Default|GetIsSpiderDead))
    (AI|AIMoveTo self "0, 0, 0" (Game|GetPlayerCharacter 0) 5.0 false :!label _label
      (:OnSuccess
        _)
      (:OnFail
        _))
    (Utilities|FlowControl|Delay 0.2)
    (goto _label)))

(event EventTick
  (params (DeltaSeconds :type Float%20%28single-precision%29))
  ;[1 0 0.1717] attack
  (if (not (Variables|Default|GetIsSpiderDead))
    (if (CallFunction|AttackRange)
      (Utilities|FlowControl|Delay 0.6)
      (Components|Activation|Deactivate (Variables|Character|GetCharacterMovement))
      (Animation|Montage|PlayMontage (Variables|Character|GetMesh) "/Game/Characters/Enemy_Great_Spider/Animations/SpiderAtack01.SpiderAtack01" 2.0
        (:OnCompleted
          (Components|Activation|Activate (Variables|Character|GetCharacterMovement) false))))))

(event Game|Damage|EventAnyDamage
  (params (Damage :type Float%20%28single-precision%29) (DamageType :type Damage%20Type%20Object%20Reference) (InstigatedBy :type Controller%20Object%20Reference) (DamageCauser :type Actor%20Object%20Reference))
  ;[1 0.1818 0] Death
  (CallFunction|ApplySpiderDamage Damage))

(fn ConstructionScript)

(fn AttackRange
  (bind _asbp_soldier (Utilities|Casting|CastToBP_Soldier (Game|Player|GetPlayerPawn 0)))
  (return (< (Transformation|GetDistanceTo _asbp_soldier) 1e+02)))

(fn IsSpiderDead01
  (params (Damage :type Float%20%28single-precision%29))
  (bind _output_get (Variables|Default|SetAlien_health (- (Variables|Default|GetAlien_health) Damage)))
  (if (== _output_get 0.0)
    _))

(fn ApplySpiderDamage
  (params (Damage :type Float%20%28single-precision%29))
  (bind _output_get (Variables|Default|SetAlien_health (- (Variables|Default|GetAlien_health) Damage)))
  (Development|PrintString (Utilities|String|ToString(Float) _output_get))
  (if (== (Math|Float|Clamp(Float) _output_get 0.0 6e+01) 0.0)
    (bind _output_get_2 (Variables|Default|SetIsSpiderDead true))
    (bind _outactors (Actor|GetAllActorsOfClass "/Game/blueprints/characters_blueprits/BP_Soldier.BP_Soldier_C"))
    (Variables|/Game/blueprints/characters_blueprits/BP_Soldier.BP_Soldier_C|SetKillCount (Utilities|Array|Get(acopy) _outactors) (+ (Variables|/Game/blueprints/characters_blueprits/BP_Soldier.BP_Soldier_C|GetKillCount (Utilities|Array|Get(acopy) _outactors)) 1.0))
    (Components|Activation|Deactivate (Variables|Character|GetCharacterMovement))
    (return _output_get_2)))