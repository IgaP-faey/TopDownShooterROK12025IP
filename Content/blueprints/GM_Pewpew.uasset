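; GM_Pewpew is the game mode that runs endless waves of alien spiders, starting shortly after play begins.
; Each wave scales the previous spider count by a difficulty multiplier, then a looping timer spawns them at random TargetPoints.
; RegisterAlienDeath removes dead spiders from the tracking array and starts the next wave after a brief delay once none remain.
; From wave three onward, every spawned spider is enlarged, with overridden health and attack distance.
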(event Custom|SpawnAlien
  (bind _returnvalue (CallFunction|EnemiesSpawn))
  (Utilities|Array|Add (Variables|Default|GetSpiderArray) _returnvalue)
  (bind _result (Math|Integer|DecrementInt (Variables|Default|GetSpiderNum2Spawn))
    (:%20%20
      (bind _output_get (Variables|Default|SetSpiderNum2Spawn _result))
      (if (== _output_get 0)
        (Utilities|Time|ClearTimerbyFunctionName 0 "SpawnAlien")))))

(event Custom|EndWave
  (Utilities|FlowControl|Delay 0.5)
  (CallFunction|StartNewWave))

(event EventBeginPlay
  ;[0.9096 0.4331 1] wave numer
  (Utilities|FlowControl|Delay 5.0)
  (CallFunction|StartNewWave))

(fn ConstructionScript)

(fn EnemiesSpawn
  (bind _outactors (Actor|GetAllActorsOfClass "/Script/Engine.TargetPoint"))
  (bind _returnvalue (Game|SpawnActorfromClass "/Game/blueprints/characters_blueprits/BP_AlienSpider.BP_AlienSpider_C" (Transformation|GetActorTransform (Utilities|Array|Get(acopy) _outactors (Math|Random|RandomIntegerinRange 0 (Utilities|Array|LastIndex _outactors)))) "Undefined" 0 0))
  (if (>= (Variables|Default|GetWaveNum) 3)
    (CallFunction|SpiderDifficulty _returnvalue))
  (return _returnvalue))

(fn RegisterAlienDeath
  (params (Item :type BP%20Alien%20Spider%20Object%20Reference%20%28by%20ref%29))
  (bind _spiderarray (Variables|Default|GetSpiderArray))
  (Utilities|Array|RemoveItem _spiderarray Item)
  (if (and (== (Utilities|Array|Length _spiderarray) 0) (== (Variables|Default|GetSpiderNum2Spawn) 0))
    (CallFunction|EndWave)))

(fn StartNewWave
  (Math|Integer|IncrementInt (Variables|Default|GetWaveNum)
    (:%20%20
      (CallFunction|DiffWave)
      (Utilities|Time|SetTimerbyFunctionName 0 "SpawnAlien" 2.0 true))))

(fn DiffWave
  (bind _output_get (Variables|Default|SetSpiderNum2Spawn (Math|Float|Round (* (Variables|Default|GetSpiderLastLvl) (Variables|Default|GetDiffLvl)))))
  (Variables|Default|SetSpiderLastLvl _output_get))

(fn SpiderDifficulty
  (params (SpawnedStrongSpider :type BP%20Alien%20Spider%20Object%20Reference))
  (bind _output_get (Variables|Default|SetSpawnedStrongSpider SpawnedStrongSpider))
  (Variables|/Game/blueprints/characters_blueprits/BP_AlienSpider.BP_AlienSpider_C|SetAlien_health _output_get 2.5e+02)
  (Transformation|SetActorScale3D _output_get (* (Transformation|GetActorScale3D _output_get) 2.0))
  (Variables|/Game/blueprints/characters_blueprits/BP_AlienSpider.BP_AlienSpider_C|SetAttackDistance _output_get 2e+02))